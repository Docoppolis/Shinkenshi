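; Game mode that holds level progression info and handles player respawning.
; On BeginPlay it copies the current and next level from the first Level_Info_BP actor in the level.
; RespawnPlayer spawns a new actor of the given player's class at the stored RespawnTransform and has player controller 0 possess it.
; RespawnTransform is not set here, and the old player actor is not destroyed here.
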(event `self.ReceiveBeginPlay`
  (bind _outactors (`GameplayStatics.GetAllActorsOfClass` "/Game/Blueprints/Misc/Level_Info_BP.Level_Info_BP_C"))
  (bind _output (`|GetArrayItem` _outactors))
  (set `self.nextLevel` (`/Game/Blueprints/Misc/Level_Info_BP.nextLevel` _output))
  (set `self.currentLevel` (`/Game/Blueprints/Misc/Level_Info_BP.currentLevel` _output)))

(event `RespawnPlayer`
  (params (Player :type "/Game/Blueprints/Player/Player_BP Object Reference"))
  (bind _returnvalue (`|SpawnActorFromClass` (`GameplayStatics.GetObjectClass` Player) (`self.respawnTransform`) "Undefined" "MultiplyWithRoot" null null))
  (`Controller.Possess` (`GameplayStatics.GetPlayerController` 0) _returnvalue))

(fn `UserConstructionScript`)