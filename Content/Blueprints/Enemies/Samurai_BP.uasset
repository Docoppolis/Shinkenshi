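; Samurai_BP is a Paper2D samurai enemy that chases and attacks Player_BP, swapping flipbooks for idle, run, attack and hurt.
; A per-tick line trace along its facing axis triggers Enemy_AI to follow the player, while LedgeDetection end-overlap halts movement until facing and player-position checks allow pursuit.
; AttackDamage overlap starts a delayed, cooldown-gated attack that damages the player and toggles hitbox collision.
; Incoming damage plays a hurt reaction and destroys the actor at zero health.
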(event `self.ReceiveAnyDamage`
  (params (Damage :type "Float (single-precision)") (DamageType :type "DamageType Object Reference") (InstigatedBy :type "Controller Object Reference") (DamageCauser :type "Actor Object Reference"))
  (bind _sprite (`self.Sprite`))
  ;[1 1 1] Take Damage
  (if (not (`self.isDead`))
    (set `self.gettingHit` true)
    (set `self.currentHealth` (`KismetMathLibrary.FClamp` (- (`self.currentHealth`) Damage) 0.0 (`self.maxHealth`)))
    (`PaperFlipbookComponent.SetLooping` (`self.Sprite`) false)
    (`PaperFlipbookComponent.SetFlipbook` _sprite "/Game/Assets/Flipbooks/Samurai/Samurai_Hurt.Samurai_Hurt")
    (`KismetSystemLibrary.Delay` 1.0)
    (`PaperFlipbookComponent.SetLooping` _sprite true)
    (`PaperFlipbookComponent.Play` _sprite)
    (if (== (`self.currentHealth`) 0.0)
      (`self.Death`)
      (else
        (`PaperFlipbookComponent.SetFlipbook` (`self.Sprite`) "/Game/Assets/Flipbooks/Samurai/Samurai_Idle.Samurai_Idle")
        (set `self.gettingHit` false)))))

(event `Death`
  ;[1 1 1] Death
  (set `self.isDead` true)
  (`self.K2_DestroyActor`))

(event `Attack Anim`
  (bind _sprite (`self.Sprite`))
  (bind _sprite_2 (`self.Sprite`))
  (`PaperFlipbookComponent.SetLooping` _sprite false)
  (`PaperFlipbookComponent.SetFlipbook` _sprite "/Game/Assets/Flipbooks/Samurai/Samurai_Attack1.Samurai_Attack1")
  (`GameplayStatics.PlaySoundAtLocation` "/Game/Assets/Sound/Movement/Enemy_Attack_SC.Enemy_Attack_SC" (`self.K2_GetActorLocation`) (struct) 1.0 1.0 0.0 null null null null)
  (`KismetSystemLibrary.Delay` 0.4)
  (`PaperFlipbookComponent.SetLooping` _sprite_2 true)
  (`PaperFlipbookComponent.Play` _sprite_2)
  (`PaperFlipbookComponent.SetFlipbook` _sprite_2 "/Game/Assets/Flipbooks/Samurai/Samurai_Idle.Samurai_Idle")
  (`KismetSystemLibrary.Delay` 1.0))

(event `Get Player Status`
  (bind _attack_damage (`self.Attack Damage`))
  (`PrimitiveComponent.SetCollisionProfileName` _attack_damage "OverlapAllDynamic" true)
  (`PrimitiveComponent.SetCollisionProfileName` _attack_damage "NoCollision" true))

(event `self.Attack Damage.OnComponentBeginOverlap`
  (params (OverlappedComponent :type "PrimitiveComponent Object Reference") (OtherActor :type "Actor Object Reference") (OtherComp :type "PrimitiveComponent Object Reference") (OtherBodyIndex :type Integer) (bFromSweep :type Boolean) (SweepResult :type "HitResult Structure (by ref)"))
  (if (not (or (`self.gettingHit`) (`self.isAttacking`)))
    (`KismetSystemLibrary.Delay` 0.5)
    (cast `/Game/Blueprints/Player/Player_BP` OtherActor)
    (`self.Attack Anim`)
    (set `self.isAttacking` true)
    (`GameplayStatics.ApplyDamage` OtherActor 1.0 null self)
    (`self.Deal Damage`)
    (`self.Stop Damage`)
    (`KismetSystemLibrary.Delay` 1.5)
    (set `self.isAttacking` false)))

(event `Deal Damage`
  (if (`self.canDealDamage`)
    (set `self.canDealDamage` false)
    (`PrimitiveComponent.SetCollisionProfileName` (`self.Attack Damage`) "OverlapAllDynamic" true)))

(event `Stop Damage`
  (`PrimitiveComponent.SetCollisionProfileName` (`self.Attack Damage`) "NoCollision" true)
  (set `self.canDealDamage` true))

(event `self.ReceiveTick`
  (params (DeltaSeconds :type "Float (single-precision)"))
  (bind _returnvalue (`self.K2_GetActorLocation` self))
  (bind _x (.x (`self.K2_GetActorLocation`)))
  (bind _returnvalue_2 (* (`KismetMathLibrary.GetForwardVector` (`self.K2_GetActorRotation` self)) 200.0))
  (if (not (`self.isAttacking`))
    (bind _outhit (`KismetSystemLibrary.LineTraceSingle` :`Start` (+ _returnvalue _returnvalue_2) :`End` (- _returnvalue _returnvalue_2) :`TraceChannel` "TraceTypeQuery1" :`DrawDebugType` "ForOneFrame"))
    (cast `/Game/Blueprints/Player/Player_BP` (`.HitActor` (`GameplayStatics.BreakHitResult` _outhit)))
    (set `self.isSeeingPlayer` true)
    (bind _asenemy_ai (cast `/Game/Blueprints/Enemies/Enemy_AI` (`self.GetController` self)))
    (if (`self.atLedge`)
      (bind _x_2 (.x (`/Game/Blueprints/Enemies/Enemy_AI.playerLocation` _asenemy_ai)))
      (if (and (== (`self.K2_GetActorRotation`) (struct :`Yaw` 180.0)) (< _x_2 _x))
        _
        (elif (not (and (== (`self.K2_GetActorRotation`) (struct)) (> _x_2 _x)))
          (`/Game/Blueprints/Enemies/Enemy_AI.Follow Player` _asenemy_ai :!label _label)
          (set `self.atLedge` false)))
      (else
        (goto _label)))))

(event `Move Anim`
  (`PaperFlipbookComponent.SetFlipbook` (`self.Sprite`) "/Game/Assets/Flipbooks/Samurai/Samurai_Run.Samurai_Run"))

(event `Stop Move Anim`
  (`PaperFlipbookComponent.SetFlipbook` (`self.Sprite`) "/Game/Assets/Flipbooks/Samurai/Samurai_Idle.Samurai_Idle"))

(event `self.Ledge Detection.OnComponentEndOverlap`
  (params (OverlappedComponent :type "PrimitiveComponent Object Reference") (OtherActor :type "Actor Object Reference") (OtherComp :type "PrimitiveComponent Object Reference") (OtherBodyIndex :type Integer))
  (set `self.atLedge` true)
  (bind _asenemy_ai (cast `/Game/Blueprints/Enemies/Enemy_AI` (`self.GetController`)))
  (`Controller.StopMovement` _asenemy_ai)
  (`self.Stop Move Anim`))

(fn `UserConstructionScript`)