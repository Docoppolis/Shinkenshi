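; Samurai2_BP is a 2D Paper flipbook samurai enemy that chases and attacks the player.
; Tick traces along its facing axis, ignoring tilemaps, and tells its Enemy_AI controller to follow a detected player, while LedgeDetection stops and flips it at edges.
; AttackDamage overlap triggers the attack animation and damages the player.
; Incoming damage plays a hurt flipbook, knocks it away from the attacker and destroys it at zero health.
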(event `self.ReceiveAnyDamage`
  (params (Damage :type "Float (single-precision)") (DamageType :type "DamageType Object Reference") (InstigatedBy :type "Controller Object Reference") (DamageCauser :type "Actor Object Reference"))
  (bind _sprite (`self.Sprite`))
  ;[1 1 1] Take Damage
  (if (not (`self.isDead`))
    (if (< (.x (`KismetMathLibrary.Normal` (- (`self.K2_GetActorLocation` DamageCauser) (`self.K2_GetActorLocation`)))) 0.0)
      (set `self.damageFromRight` false)
      (else
        (set `self.damageFromRight` true)))
    (set `self.gettingHit` true)
    (set `self.currentHealth` (`KismetMathLibrary.FClamp` (- (`self.currentHealth`) Damage) 0.0 (`self.maxHealth`)))
    (`PaperFlipbookComponent.SetLooping` (`self.Sprite`) false)
    (`PaperFlipbookComponent.SetFlipbook` _sprite "/Game/Assets/Flipbooks/Samurai2/Samurai2_Hurt.Samurai2_Hurt")
    (if (`self.damageFromRight`)
      (`self.LaunchCharacter` (-300.0 0.0 0.0))
      (else
        (`self.LaunchCharacter` (300.0 0.0 0.0))))
    (`KismetSystemLibrary.Delay` 0.7)
    (`PaperFlipbookComponent.SetLooping` _sprite true)
    (`PaperFlipbookComponent.Play` _sprite)
    (if (== (`self.currentHealth`) 0.0)
      (`self.Death`)
      (else
        (`PaperFlipbookComponent.SetFlipbook` (`self.Sprite`) "/Game/Assets/Flipbooks/Samurai2/Samurai2_Idle.Samurai2_Idle")
        (set `self.gettingHit` false)))))

(event `Death`
  ;[1 1 1] Death
  (set `self.isDead` true)
  (`self.K2_DestroyActor`))

(event `Attack Anim`
  (bind _sprite (`self.Sprite`))
  (bind _sprite_2 (`self.Sprite`))
  (set `self.isAttacking` true)
  (`PaperFlipbookComponent.SetLooping` _sprite false)
  (`PaperFlipbookComponent.SetFlipbook` _sprite "/Game/Assets/Flipbooks/Samurai2/Samurai2_Attack.Samurai2_Attack")
  (`GameplayStatics.PlaySoundAtLocation` "/Game/Assets/Sound/Movement/Enemy_Attack_SC.Enemy_Attack_SC" (`self.K2_GetActorLocation`) (struct) 1.0 1.0 0.0 null null null null)
  (`KismetSystemLibrary.Delay` 0.4)
  (`PaperFlipbookComponent.SetLooping` _sprite_2 true)
  (`PaperFlipbookComponent.Play` _sprite_2)
  (`PaperFlipbookComponent.SetFlipbook` _sprite_2 "/Game/Assets/Flipbooks/Samurai2/Samurai2_Idle.Samurai2_Idle")
  (`KismetSystemLibrary.Delay` 1.0)
  (set `self.isAttacking` false))

(event `Get Player Status`
  (bind _attack_damage (`self.Attack Damage`))
  (`PrimitiveComponent.SetCollisionProfileName` _attack_damage "OverlapAllDynamic" true)
  (`PrimitiveComponent.SetCollisionProfileName` _attack_damage "NoCollision" true))

(event `Deal Damage`
  (if (`self.canDealDamage`)
    (`PrimitiveComponent.SetCollisionProfileName` (`self.Attack Damage`) "OverlapAllDynamic" true)))

(event `Stop Damage`
  (`PrimitiveComponent.SetCollisionProfileName` (`self.Attack Damage`) "NoCollision" true))

(event `self.Attack Damage.OnComponentBeginOverlap`
  (params (OverlappedComponent :type "PrimitiveComponent Object Reference") (OtherActor :type "Actor Object Reference") (OtherComp :type "PrimitiveComponent Object Reference") (OtherBodyIndex :type Integer) (bFromSweep :type Boolean) (SweepResult :type "HitResult Structure (by ref)"))
  (cast `/Game/Blueprints/Player/Player_BP` OtherActor)
  (set `self.canDealDamage` false)
  (`self.Attack Anim`)
  (`GameplayStatics.ApplyDamage` OtherActor 1.0 null self)
  (`self.Deal Damage`)
  (`self.Stop Damage`)
  (`KismetSystemLibrary.Delay` 0.4)
  (set `self.canDealDamage` true))

(event `self.ReceiveTick`
  (params (DeltaSeconds :type "Float (single-precision)"))
  (bind _returnvalue (`self.K2_GetActorLocation` self))
  (bind _x (.x (`self.K2_GetActorLocation`)))
  (bind _returnvalue_2 (* (`KismetMathLibrary.GetForwardVector` (`self.K2_GetActorRotation` self)) 200.0))
  (if (not (or (`self.isAttacking`) (`self.gettingHit`)))
    (bind _outactors (`GameplayStatics.GetAllActorsOfClass` "/Script/Paper2D.PaperTileMapActor"))
    (bind _outhit (`KismetSystemLibrary.LineTraceSingle` (+ _returnvalue _returnvalue_2) (- _returnvalue _returnvalue_2) "TraceTypeQuery1" false _outactors "ForOneFrame"))
    (cast `/Game/Blueprints/Player/Player_BP` (`.HitActor` (`GameplayStatics.BreakHitResult` _outhit)))
    (set `self.isSeeingPlayer` true)
    (bind _asenemy_ai (cast `/Game/Blueprints/Enemies/Enemy_AI` (`self.GetController` self)))
    (if (`self.atLedge`)
      (bind _x_2 (.x (`/Game/Blueprints/Enemies/Enemy_AI.playerLocation` _asenemy_ai)))
      (if (and (== (`self.K2_GetActorRotation`) (struct :`Yaw` 180.0)) (< _x_2 _x))
        _
        (elif (not (and (== (`self.K2_GetActorRotation`) (struct)) (> _x_2 _x)))
          (`/Game/Blueprints/Enemies/Enemy_AI.Follow Player` _asenemy_ai :!label _label)))
      (else
        (goto _label)))))

(event `Move Anim`
  (`PaperFlipbookComponent.SetFlipbook` (`self.Sprite`) "/Game/Assets/Flipbooks/Samurai2/Samurai2_Run.Samurai2_Run"))

(event `Stop Move Anim`
  (`PaperFlipbookComponent.SetFlipbook` (`self.Sprite`) "/Game/Assets/Flipbooks/Samurai2/Samurai2_Idle.Samurai2_Idle"))

(event `self.Ledge Detection.OnComponentEndOverlap`
  (params (OverlappedComponent :type "PrimitiveComponent Object Reference") (OtherActor :type "Actor Object Reference") (OtherComp :type "PrimitiveComponent Object Reference") (OtherBodyIndex :type Integer))
  (set `self.atLedge` true)
  (bind _asenemy_ai (cast `/Game/Blueprints/Enemies/Enemy_AI` (`self.GetController`)))
  (`Controller.StopMovement` _asenemy_ai)
  (`self.Stop Move Anim`)
  (if (== (`self.K2_GetActorRotation`) (struct :`Yaw` 180.0))
    (`self.K2_SetActorRotation` (struct))
    (else
      (`self.K2_SetActorRotation` (struct :`Yaw` 180.0))))
  (`KismetSystemLibrary.Delay` 0.5)
  (set `self.atLedge` false))

(fn `UserConstructionScript`)