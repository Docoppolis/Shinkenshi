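; Paper2D boar enemy that walks forward every tick unless attacking and turns around when its WallDetector overlaps something.
; An AttackDamage overlap triggers a timed attack flipbook and applies damage to a living Player_BP.
; Incoming damage lowers clamped health and destroys the boar at zero.
; The forward trace result and attack cooldown flag are never read, and DealDamage and StopDamage set the same collision profile.
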(event `self.ReceiveBeginPlay`)

(event `self.ReceiveTick`
  (params (DeltaSeconds :type "Float (single-precision)"))
  (bind _returnvalue (`self.K2_GetActorLocation` self))
  (if (not (`self.isAttacking`))
    (bind _outhit (`KismetSystemLibrary.LineTraceSingle` :`Start` _returnvalue :`End` (+ _returnvalue (* (`KismetMathLibrary.GetForwardVector` (`self.K2_GetActorRotation` self)) 500.0)) :`TraceChannel` "TraceTypeQuery1" :`DrawDebugType` "ForOneFrame"))
    (`self.AddMovementInput` (`KismetMathLibrary.GetForwardVector` (`self.K2_GetActorRotation`)))))

(event `Attack`
  (bind _sprite (`self.Sprite`))
  (bind _sprite_2 (`self.Sprite`))
  ;[1 1 1] Attack
  (if (not (`self.gettingHit`))
    (`self.Deal Damage`)
    (`self.Stop Damage`)
    (if (not (`self.isAttacking`))
      (set `self.isAttacking` true)
      (`PaperFlipbookComponent.SetLooping` _sprite false)
      (`PaperFlipbookComponent.SetFlipbook` _sprite "/Game/Assets/Flipbooks/Boar/Boar_Attack.Boar_Attack")
      (`KismetSystemLibrary.Delay` 0.4)
      (`PaperFlipbookComponent.SetLooping` _sprite_2 true)
      (`PaperFlipbookComponent.Play` _sprite_2)
      (`PaperFlipbookComponent.SetFlipbook` (`self.Sprite`) "/Game/Assets/Flipbooks/Boar/Boar_Run.Boar_Run")
      (set `self.isAttacking` false)
      (set `self.attackOnCD` true)
      (`KismetSystemLibrary.Delay` 0.4)
      (set `self.attackOnCD` false))))

(event `Deal Damage`
  ;[1 1 1] Attack
  (if (`self.canDealDamage`)
    (`PrimitiveComponent.SetCollisionProfileName` (`self.Attack Damage`) "OverlapOnlyPawn" true)))

(event `Stop Damage`
  ;[1 1 1] Attack
  (`PrimitiveComponent.SetCollisionProfileName` (`self.Attack Damage`) "OverlapOnlyPawn" true))

(event `self.Attack Damage.OnComponentBeginOverlap`
  (params (OverlappedComponent :type "PrimitiveComponent Object Reference") (OtherActor :type "Actor Object Reference") (OtherComp :type "PrimitiveComponent Object Reference") (OtherBodyIndex :type Integer) (bFromSweep :type Boolean) (SweepResult :type "HitResult Structure (by ref)"))
  ;[1 1 1] Attack
  (`KismetSystemLibrary.PrintString` (`KismetStringLibrary.Conv_IntToString` (`self.overlapCount`)))
  (set `self.canDealDamage` false)
  (`self.Attack`)
  (bind _asplayer_bp (cast `/Game/Blueprints/Player/Player_BP` OtherActor))
  (if (`/Game/Blueprints/Player/Player_BP.isDead` _asplayer_bp)
    (set `self.isPlayerDead` true)
    (else
      (set `self.isPlayerDead` false)
      (`GameplayStatics.ApplyDamage` OtherActor 1.0 null self)
      (`KismetSystemLibrary.Delay` 0.4)))
  (set `self.canDealDamage` true)
  (set `self.overlapCount` (+ (`self.overlapCount`) 1)))

(event `self.Wall Detector.OnComponentBeginOverlap`
  (params (OverlappedComponent :type "PrimitiveComponent Object Reference") (OtherActor :type "Actor Object Reference") (OtherComp :type "PrimitiveComponent Object Reference") (OtherBodyIndex :type Integer) (bFromSweep :type Boolean) (SweepResult :type "HitResult Structure (by ref)"))
  ;[1 1 1] Wall Detection
  (`self.turnCharacter`))

(event `self.ReceiveAnyDamage`
  (params (Damage :type "Float (single-precision)") (DamageType :type "DamageType Object Reference") (InstigatedBy :type "Controller Object Reference") (DamageCauser :type "Actor Object Reference"))
  ;[1 1 1] Take Damage
  (if (not (`self.isDead`))
    (set `self.gettingHit` true)
    (set `self.currentHealth` (`KismetMathLibrary.FClamp` (- (`self.currentHealth`) Damage) 0.0 (`self.maxHealth`)))
    (if (== (`self.currentHealth`) 0.0)
      (`self.Death`)
      (else
        (`PaperFlipbookComponent.SetFlipbook` (`self.Sprite`) "/Game/Assets/Flipbooks/Boar/Boar_Run.Boar_Run")
        (set `self.gettingHit` false)))))

(event `Death`
  ;[1 1 1] Take Damage
  (set `self.isDead` true)
  (`self.K2_DestroyActor`))

(fn `turnCharacter`
  (`self.K2_SetActorRotation` (`KismetMathLibrary.ComposeRotators` (`self.K2_GetActorRotation`) (struct :`Yaw` 180.0))))

(fn `UserConstructionScript`)