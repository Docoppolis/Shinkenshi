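; BP_CameraPawn is an auto-scrolling camera pawn for the bamboo tileset content.
; On BeginPlay it spawns a foreground actor and four background layer actors at its own location, then destroys the actors in SampleTilemaps.
; Each Tick it moves along its right vector at MoveSpeed, scaled by delta time, while its X position stays below a fixed limit.
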(event `self.ReceiveBeginPlay`
  (bind _returnvalue (`self.K2_GetActorLocation`))
  (`|SpawnActorFromClass` "/Game/Assets/BambooTilesetContent/Blueprints/BP_Foreground.BP_Foreground_C" (`KismetMathLibrary.MakeTransform` (`self.K2_GetActorLocation`)) "Undefined" "MultiplyWithRoot" null null)
  (`|SpawnActorFromClass` "/Game/Assets/BambooTilesetContent/Blueprints/BP_Background_1.BP_Background_1_C" (`KismetMathLibrary.MakeTransform` _returnvalue) "Undefined" "MultiplyWithRoot" null null)
  (`|SpawnActorFromClass` "/Game/Assets/BambooTilesetContent/Blueprints/BP_Background_2.BP_Background_2_C" (`KismetMathLibrary.MakeTransform` _returnvalue) "Undefined" "MultiplyWithRoot" null null)
  (`|SpawnActorFromClass` "/Game/Assets/BambooTilesetContent/Blueprints/BP_Background_3.BP_Background_3_C" (`KismetMathLibrary.MakeTransform` (`self.K2_GetActorLocation`)) "Undefined" "MultiplyWithRoot" null null)
  (`|SpawnActorFromClass` "/Game/Assets/BambooTilesetContent/Blueprints/BP_Background_4.BP_Background_4_C" (`KismetMathLibrary.MakeTransform` (`self.K2_GetActorLocation`)) "Undefined" "MultiplyWithRoot" null null)
  (for _array_element (`self.sampleTilemaps`)
    (`self.K2_DestroyActor` _array_element)))

(event `self.ReceiveTick`
  (params (DeltaSeconds :type "Float (single-precision)"))
  (bind _returnvalue_x (`KismetMathLibrary.BreakVector` (`self.K2_GetActorLocation`)))
  (if (< _returnvalue_x 1210.0)
    (`self.K2_SetActorLocation` (+ (`self.K2_GetActorLocation`) (* (`self.GetActorRightVector`) (* (`GameplayStatics.GetWorldDeltaSeconds`) (`self.moveSpeed`)))))))

(fn `UserConstructionScript`)